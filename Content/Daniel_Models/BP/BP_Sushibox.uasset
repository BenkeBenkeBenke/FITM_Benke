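; Sushi box actor that rides as a cart along the spline of a referenced track.
; SendPackage calls MoveCart when ActiveCar is set; if IsOmw, a timeline plays at a rate derived from Duration.
; Its alpha maps to spline distance, setting world location and rotation; CarStartOffset sets the timeline time, but PlayFromStart then restarts it.
; Box overlap is empty, and the "Stop" tag check that clears IsOmw is disconnected.
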(event `/Game/Daniel_UI/Score_Interface.SendPackage`
  (params (Send :type Boolean))
  (if (`self.ActiveCar`)
    (`self.MoveCart`)))

(event `MoveCart`
  (bind _returnvalue (`KismetMathLibrary.Lerp` 0.0 (`SplineComponent.GetSplineLength` (`/Game/Daniel_Models/BP/BP_Track.Spline` (`self.TrackRef`))) (`self.Alpha`)))
  (if (`self.IsOmw`)
    (`TimelineComponent.SetPlayRate` (`self.Timeline_0`) (/ 1.0 (`self.Duration`)))
    (`TimelineComponent.SetNewTime` (`self.Timeline_0`) (`self.CarStartOffset`))
    (bind (_direction _newtrack_1) (`Timeline|Timeline_0` :!via `PlayFromStart`)
      (:`Update`
        (set `self.Alpha` _newtrack_1)
        (`self.K2_SetActorLocationAndRotation` (`SplineComponent.GetLocationAtDistanceAlongSpline` (`/Game/Daniel_Models/BP/BP_Track.Spline` (`self.TrackRef`)) _returnvalue "World") (`SplineComponent.GetRotationAtDistanceAlongSpline` (`/Game/Daniel_Models/BP/BP_Track.Spline` (`self.TrackRef`)) _returnvalue "World"))))))

(event `self.Box.OnComponentBeginOverlap`
  (params (OverlappedComponent :type "PrimitiveComponent Object Reference") (OtherActor :type "Actor Object Reference") (OtherComp :type "PrimitiveComponent Object Reference") (OtherBodyIndex :type Integer) (bFromSweep :type Boolean) (SweepResult :type "HitResult Structure (by ref)")))

(fn `UserConstructionScript`)