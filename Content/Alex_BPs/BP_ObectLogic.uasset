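; Moving object actor that slides along negative world Y, with sweep, at a speed set through an event.
; BeginPlay messages the game instance with itself as sender; CustomEvent stores and prints the new speed.
; Each Tick, a persistently drawn 60-unit trace toward positive Y, opposite to travel, halts movement on hitting an actor other than BP_Test and resumes it when clear.
; GoorNoGo also re-enables movement; the box overlap handlers are empty.
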(event `self.ReceiveTick`
  (params (DeltaSeconds :type "Float (single-precision)"))
  (bind (_returnvalue_x _returnvalue_y _returnvalue_z) (`KismetMathLibrary.BreakVector` (`self.K2_GetActorLocation`)))
  (bind (_returnvalue_x_2 _returnvalue_y_2 _returnvalue_z_2) (`KismetMathLibrary.BreakVector` (`self.K2_GetActorLocation` self)))
  (if (`self.MayIMove?`)
    (`self.K2_SetActorLocation` (`KismetMathLibrary.MakeVector` _returnvalue_x (- _returnvalue_y (* DeltaSeconds (`self.SpeedInObject`))) _returnvalue_z) true))
  (if (`KismetSystemLibrary.IsValid` self)
    (bind _outhit (`KismetSystemLibrary.LineTraceSingle` (`KismetMathLibrary.MakeVector` _returnvalue_x_2 _returnvalue_y_2 _returnvalue_z_2) (`KismetMathLibrary.MakeVector` _returnvalue_x_2 (+ _returnvalue_y_2 60.0) _returnvalue_z_2) "TraceTypeQuery3" false (`|MakeArray` self) "Persistent"))
    (bind (_bblockinghit _binitialoverlap _time _distance _location _impactpoint _normal _impactnormal _physmat _hitactor) (`GameplayStatics.BreakHitResult` _outhit))
    (if (!= _hitactor "/Game/Alex_BPs/BP_Test.BP_Test")
      (if (`KismetSystemLibrary.IsValid` _hitactor)
        (set `self.MayIMove?` false)
        (else
          (set `self.MayIMove?` true))))))

(event `self.ReceiveBeginPlay`
  (message `/Game/Alex_BPs/INT_InstanceObject.NewFunction_0` (`GameplayStatics.GetGameInstance`) 0.0 self))

(event `CustomEvent`
  (params (NewSpeed :type "Float (double-precision)") (`I sent the message` :type "Actor Object Reference"))
  (bind _output_get (set `self.SpeedInObject` NewSpeed))
  (`KismetSystemLibrary.PrintString` (`KismetStringLibrary.Conv_DoubleToString` _output_get)))

(event `self.Box1.OnComponentBeginOverlap`
  (params (OverlappedComponent :type "PrimitiveComponent Object Reference") (OtherActor :type "Actor Object Reference") (OtherComp :type "PrimitiveComponent Object Reference") (OtherBodyIndex :type Integer) (bFromSweep :type Boolean) (SweepResult :type "HitResult Structure (by ref)")))

(event `self.Box1.OnComponentEndOverlap`
  (params (OverlappedComponent :type "PrimitiveComponent Object Reference") (OtherActor :type "Actor Object Reference") (OtherComp :type "PrimitiveComponent Object Reference") (OtherBodyIndex :type Integer)))

(event `/Game/Alex_BPs/INT_PlayerObject.GoOrNoGo`
  (params (Go :type Boolean))
  (set `self.MayIMove?` true))

(fn `UserConstructionScript`)