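; BP_ObjectLauncher is a timed spawner that launches one of three random actor classes at a set spawn location with increasing frequency.
; Tick accumulates time until a randomized interval elapses, then spawns, rerolls the interval and shrinks its range by 10% until the maximum bottoms out.
; Once the minimum interval is low enough, a random cluster roll can add a second simultaneous spawn, relying on collision adjustment to separate overlapping actors.
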(event `self.ReceiveTick`
  (params (DeltaSeconds :type "Float (single-precision)"))
  (bind (_spawnlocation_x _spawnlocation_y _spawnlocation_z) (`KismetMathLibrary.BreakVector` (`self.SpawnLocation`)))
  (bind _output (`|GetArrayItem` (`|MakeArray` (`self.NewVar_1`) (`self.NewVar_2`) (`self.NewVar_3`)) (`KismetMathLibrary.RandomIntegerInRange` 0 2)))
  (bind _output_get (set `self.Count` (+ (* DeltaSeconds 1.0) (`self.Count`))))
  (if (>= _output_get (`self.SpawnRate`))
    (if (<= (`self.SpawnRateMin`) 2.0)
      (if (<= (`KismetMathLibrary.RandomFloatInRange` 1.0 100.0) (`self.ClusterOdds`))
        (`|ExecutionSequence`
          (:`then_0`
            (`|SpawnActorFromClass` _output (`KismetMathLibrary.MakeTransform` (`KismetMathLibrary.MakeVector` _spawnlocation_x _spawnlocation_y _spawnlocation_z)) "AdjustIfPossibleButDontSpawnIfColliding" "OverrideRootScale" null null))
          (:`then_1`
            (`|SpawnActorFromClass` _output (`KismetMathLibrary.MakeTransform` (`self.SpawnLocation`)) "AdjustIfPossibleButDontSpawnIfColliding" "OverrideRootScale" null null :!label _label)
            (set `self.SpawnRate` (`KismetMathLibrary.RandomFloatInRange` (`self.SpawnRateMin`) (`self.SpawnRateMax`)))
            (if (not (<= (`self.SpawnRateMax`) 1.5))
              (set `self.SpawnRateMax` (* (`self.SpawnRateMax`) 0.9))
              (set `self.SpawnRateMin` (* (`self.SpawnRateMin`) 0.9)))
            (set `self.Count` 0.0)))
        (else
          (goto _label)))
      (else
        (goto _label)))))

(fn `UserConstructionScript`)