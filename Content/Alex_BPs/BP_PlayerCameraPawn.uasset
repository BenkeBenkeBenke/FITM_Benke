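; Player camera pawn that sorts traced objects left or right with mouse clicks and tracks the total score.
; Tick traces up from a plane to store the target, which clicks shift along X from zero before sending it GoOrNoGoMessage.
; Score events adjust the total and animate the HUD.
; At -500 or below, Tick flags game over on FirstPersonGameMode, shows the fired UI and notifies Score_Interface actors.
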(event `/Game/Daniel_UI/Score_Interface.SingleScoreINT`
  (params (Scored :type Boolean))
  ;[1 1 1] Score
  (bind _foundwidgets (`WidgetBlueprintLibrary.GetAllWidgetsOfClass` "/Game/Daniel_UI/HUD.HUD_C"))
  (`/Game/Daniel_UI/HUD.ScoreAnim` _foundwidgets)
  (set `self.TotalScore` (+ (`self.TotalScore`) (`self.SingleScore`))))

(event `/Game/Daniel_UI/Score_Interface.BooScoreINT`
  (params (Scored :type Boolean))
  ;[1 1 1] Score
  (bind _foundwidgets (`WidgetBlueprintLibrary.GetAllWidgetsOfClass` "/Game/Daniel_UI/HUD.HUD_C"))
  (`/Game/Daniel_UI/HUD.ScoreAnim` _foundwidgets)
  (set `self.TotalScore` (- (`self.TotalScore`) (`self.ReduceScore`)))
  (`KismetSystemLibrary.PrintString` ""))

(event `/Game/Daniel_UI/Score_Interface.NotCompleteScoreINT`
  (params (Scored :type Boolean))
  ;[1 1 1] Score
  (bind _foundwidgets (`WidgetBlueprintLibrary.GetAllWidgetsOfClass` "/Game/Daniel_UI/HUD.HUD_C"))
  (`/Game/Daniel_UI/HUD.ScoreAnim` _foundwidgets)
  (set `self.TotalScore` (- (`self.TotalScore`) (`self.NotCompleteScore`)))
  (`KismetSystemLibrary.PrintString` ""))

(event `/Game/Daniel_UI/Score_Interface.CompleteScoreINT`
  (params (Scored :type Boolean))
  ;[1 1 1] Score
  (bind _foundwidgets (`WidgetBlueprintLibrary.GetAllWidgetsOfClass` "/Game/Daniel_UI/HUD.HUD_C"))
  (`/Game/Daniel_UI/HUD.ScoreAnim` _foundwidgets)
  (set `self.TotalScore` (+ (`self.TotalScore`) (`self.CompeteScore`)))
  (`KismetSystemLibrary.PrintString` ""))

(event `self.ReceiveTick`
  (params (DeltaSeconds :type "Float (single-precision)"))
  (bind (_returnvalue_x _returnvalue_y _returnvalue_z) (`KismetMathLibrary.BreakVector` (`SceneComponent.K2_GetComponentLocation` (`self.Plane`))))
  (`|ExecutionSequence`
    (:`then_0`
      (bind (_outhit _returnvalue) (`KismetSystemLibrary.LineTraceSingle` :`Start` (`KismetMathLibrary.MakeVector` _returnvalue_x _returnvalue_y _returnvalue_z) :`End` (`KismetMathLibrary.MakeVector` _returnvalue_x _returnvalue_y (+ _returnvalue_z 100.0)) :`TraceChannel` "TraceTypeQuery1" :`DrawDebugType` "Persistent"))
      (if _returnvalue
        (set `self.TargetObject` (`.HitActor` (`GameplayStatics.BreakHitResult` _outhit)))))
    (:`then_1`
      ;[1 1 1] EndGame
      (if (<= (`self.TotalScore`) -500)
        (`/Engine/EditorBlueprintResources/StandardMacros.DoOnce` false
          (:`Completed`
            (bind _asfirst_person_game_mode (cast `/Game/FirstPersonBP/Blueprints/FirstPersonGameMode` (`GameplayStatics.GetGameMode`)))
            (set `/Game/FirstPersonBP/Blueprints/FirstPersonGameMode.GameOver` true _asfirst_person_game_mode)
            (bind _foundwidgets (`WidgetBlueprintLibrary.GetAllWidgetsOfClass` "/Game/Daniel_UI/HUD.HUD_C"))
            (`/Game/Daniel_UI/HUD.FiredUI` _foundwidgets)
            (bind _outactors (`GameplayStatics.GetAllActorsWithInterface` "/Game/Daniel_UI/Score_Interface.Score_Interface_C"))
            (for _array_element _outactors
              (message `/Game/Daniel_UI/Score_Interface.EndGame` _array_element false))))))))

(event `/Game/Daniel_UI/Score_Interface.EndGame`
  (params (EndGame :type Boolean))
  ;[1 1 1] 10/10 Smart boi me, best code 2020 - Daniel
  (set `self.GameOver` true))

(event `Key|RightMouseButton`
  (params (Key :type "Key Structure"))
  (bind _targetobject (`self.TargetObject`))
  (bind (_returnvalue_x _returnvalue_y _returnvalue_z) (`KismetMathLibrary.BreakVector` (`self.K2_GetActorLocation` _targetobject)))
  (bind _returnvalue_x_2 (`KismetMathLibrary.BreakVector` (`self.K2_GetActorLocation` _targetobject)))
  (:`Pressed`
    (if (not (`self.GameOver`))
      (`/Engine/EditorBlueprintResources/StandardMacros.IsValid` _targetobject
        (:`Is Valid`
          (if (== _returnvalue_x_2 0.0)
            (`self.K2_SetActorLocation` _targetobject (`KismetMathLibrary.MakeVector` (+ _returnvalue_x -300.0) _returnvalue_y _returnvalue_z) true false)
            (message `/Game/Alex_BPs/INT_PlayerObject.GoOrNoGo` _targetobject true :!label _label)))))))

(event `Key|LeftMouseButton`
  (params (Key :type "Key Structure"))
  (bind _targetobject (`self.TargetObject`))
  (bind _returnvalue_x (`KismetMathLibrary.BreakVector` (`self.K2_GetActorLocation` _targetobject)))
  (bind (_returnvalue_x_2 _returnvalue_y _returnvalue_z) (`KismetMathLibrary.BreakVector` (`self.K2_GetActorLocation` _targetobject)))
  (:`Pressed`
    (if (not (`self.GameOver`))
      (`/Engine/EditorBlueprintResources/StandardMacros.IsValid` _targetobject
        (:`Is Valid`
          (if (== _returnvalue_x 0.0)
            (`self.K2_SetActorLocation` _targetobject (`KismetMathLibrary.MakeVector` (+ _returnvalue_x_2 300.0) _returnvalue_y _returnvalue_z) true false)
            (goto _label)))))))

(fn `UserConstructionScript`)