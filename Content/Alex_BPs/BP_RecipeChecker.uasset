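; Recipe checker actor that picks a random recipe of colored ingredient classes and checks ingredients dropped into its box trigger.
; Four planes show the remaining ingredients through materials, and a joined class-name string is built for the widget.
; Overlapping actors are destroyed; matches leave the recipe and notify recipe-widget and score actors via interfaces.
; Once the ingredient count reaches the recipe size, it prints the result and rerolls.
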(event `self.ReceiveBeginPlay`
  (bind _plane (`self.Plane`))
  (bind _plane1 (`self.Plane1`))
  (bind _plane2 (`self.Plane2`))
  (bind _plane3 (`self.Plane3`))
  (set `self.RecipeTest_3` (`|MakeArray` "/Game/Alex_BPs/Pink.Pink_C" "/Game/Alex_BPs/Pink.Pink_C" "/Game/Alex_BPs/Gray.Gray_C" :!type "Actor Class Reference"))
  (set `self.RecipeTest_4` (`|MakeArray` "/Game/Alex_BPs/Gray.Gray_C" "/Game/Alex_BPs/Gray.Gray_C" "/Game/Alex_BPs/Gray.Gray_C" :!type "Actor Class Reference"))
  (set `self.RecipeTest_5` (`|MakeArray` "/Game/Alex_BPs/Blue.Blue_C" "/Game/Alex_BPs/Gray.Gray_C" :!type "Actor Class Reference"))
  (set `self.RecipeTest_6` (`|MakeArray` "/Game/Alex_BPs/Pink.Pink_C" "/Game/Alex_BPs/Pink.Pink_C" :!type "Actor Class Reference"))
  (bind _output_get (set `self.Recipe` (cast `/Game/Alex_BPs/NewUserDefinedEnum` (`KismetMathLibrary.Conv_IntToByte` (`KismetMathLibrary.RandomIntegerInRange` 0 (- (enumcount `/Game/Alex_BPs/NewUserDefinedEnum`) 1)))) :!label _label))
  (switch `/Game/Alex_BPs/NewUserDefinedEnum` _output_get
    (:`NewEnumerator0`
      (bind _output_get_2 (set `self.CurrentRecipe` (`self.RecipeTest_0`)))
      (`self.WidgetNameString` _output_get_2))
    (:`NewEnumerator1`
      (bind _output_get_3 (set `self.CurrentRecipe` (`self.RecipeTest_1`)))
      (`self.WidgetNameString` _output_get_3))
    (:`NewEnumerator2`
      (bind _output_get_4 (set `self.CurrentRecipe` (`self.RecipeTest_2`)))
      (`self.WidgetNameString` _output_get_4))
    (:`NewEnumerator3`
      (bind _output_get_5 (set `self.CurrentRecipe` (`self.RecipeTest_3`)))
      (`self.WidgetNameString` _output_get_5))
    (:`NewEnumerator4`
      (bind _output_get_6 (set `self.CurrentRecipe` (`self.RecipeTest_4`)))
      (`self.WidgetNameString` _output_get_6))
    (:`NewEnumerator5`
      (bind _output_get_7 (set `self.CurrentRecipe` (`self.RecipeTest_5`)))
      (`self.WidgetNameString` _output_get_7))
    (:`NewEnumerator6`
      (bind _output_get_8 (set `self.CurrentRecipe` (`self.RecipeTest_6`)))
      (`self.WidgetNameString` _output_get_8)))
  (`PrimitiveComponent.SetMaterial` (`self.Plane`) 0 "/DatasmithContent/Materials/FBXImporter/VRED/Glass.Glass" :!label _label_2)
  (`PrimitiveComponent.SetMaterial` (`self.Plane1`) 0 "/DatasmithContent/Materials/FBXImporter/VRED/Glass.Glass")
  (`PrimitiveComponent.SetMaterial` (`self.Plane2`) 0 "/DatasmithContent/Materials/FBXImporter/VRED/Glass.Glass")
  (`PrimitiveComponent.SetMaterial` (`self.Plane3`) 0 "/DatasmithContent/Materials/FBXImporter/VRED/Glass.Glass")
  (for (_array_element _array_index) (`self.CurrentRecipe`)
    (switch `int` _array_index
      (:`0`
        (bind _returnvalue (`KismetSystemLibrary.GetClassDisplayName` _array_element))
        (switch `string` _returnvalue
          (:`Gray_C`
            (`PrimitiveComponent.SetMaterial` _plane 0 "/Engine/MapTemplates/Materials/BasicAsset02.BasicAsset02"))
          (:`Pink_C`
            (`PrimitiveComponent.SetMaterial` _plane 0 "/Engine/EditorMaterials/GeometryCollection/InMaterial.InMaterial"))
          (:`Blue_C`
            (`PrimitiveComponent.SetMaterial` _plane 0 "/DatasmithContent/Materials/FBXImporter/DeltaGenMasterClearCoat.DeltaGenMasterClearCoat"))))
      (:`1`
        (switch `string` _returnvalue
          (:`Gray_C`
            (`PrimitiveComponent.SetMaterial` _plane1 0 "/Engine/MapTemplates/Materials/BasicAsset02.BasicAsset02"))
          (:`Pink_C`
            (`PrimitiveComponent.SetMaterial` _plane1 0 "/Engine/EditorMaterials/GeometryCollection/InMaterial.InMaterial"))
          (:`Blue_C`
            (`PrimitiveComponent.SetMaterial` _plane1 0 "/DatasmithContent/Materials/FBXImporter/DeltaGenMasterClearCoat.DeltaGenMasterClearCoat"))))
      (:`2`
        (switch `string` _returnvalue
          (:`Gray_C`
            (`PrimitiveComponent.SetMaterial` _plane2 0 "/Engine/MapTemplates/Materials/BasicAsset02.BasicAsset02"))
          (:`PInk_C`
            (`PrimitiveComponent.SetMaterial` _plane2 0 "/Engine/EditorMaterials/GeometryCollection/InMaterial.InMaterial"))
          (:`Blue_C`
            (`PrimitiveComponent.SetMaterial` _plane2 0 "/DatasmithContent/Materials/FBXImporter/DeltaGenMasterClearCoat.DeltaGenMasterClearCoat"))))
      (:`3`
        (switch `string` _returnvalue
          (:`Gray_C`
            (`PrimitiveComponent.SetMaterial` _plane3 0 "/Engine/MapTemplates/Materials/BasicAsset02.BasicAsset02"))
          (:`Pink_C`
            (`PrimitiveComponent.SetMaterial` _plane3 0 "/Engine/EditorMaterials/GeometryCollection/InMaterial.InMaterial")))))))

(event `CustomEvent_0`
  (goto _label))

(event `self.Box.OnComponentBeginOverlap`
  (params (OverlappedComponent :type "PrimitiveComponent Object Reference") (OtherActor :type "Actor Object Reference") (OtherComp :type "PrimitiveComponent Object Reference") (OtherBodyIndex :type Integer) (bFromSweep :type Boolean) (SweepResult :type "HitResult Structure (by ref)"))
  (bind _currentrecipe (`self.CurrentRecipe`))
  (bind _returnvalue (`KismetArrayLibrary.Array_Find` _currentrecipe (`GameplayStatics.GetObjectClass` OtherActor)))
  (`/Engine/EditorBlueprintResources/StandardMacros.DoOnce` false :!label _label_3
    (:`Completed`
      (`|ExecutionSequence`
        (:`then_0`
          (set `self.IngredientCount` (+ (`self.IngredientCount`) 1))
          (if (!= _returnvalue -1)
            (`KismetArrayLibrary.Array_Remove` _currentrecipe _returnvalue)
            (`KismetArrayLibrary.Array_Clear` (`self.IngredientStringArray`))
            (for _array_element (`self.CurrentRecipe`)
              (`KismetArrayLibrary.Array_Add` (`self.IngredientStringArray`) (`KismetSystemLibrary.GetClassDisplayName` _array_element))
              (goto _label_2))
            (set `self.CurrentRecipeWidget` (`KismetStringLibrary.JoinStringArray` (`self.IngredientStringArray`)))
            (bind _outactors (`GameplayStatics.GetAllActorsWithInterface` "/Game/Alex_BPs/INT_RecipeCheckerWidget.INT_RecipeCheckerWidget_C"))
            (for _array_element_2 _outactors
              (message `/Game/Alex_BPs/INT_RecipeCheckerWidget.IngredientAdded` _array_element_2 self))
            (bind _outactors_2 (`GameplayStatics.GetAllActorsWithInterface` "/Game/UI/Score_Interface.Score_Interface_C"))
            (for _array_element_3 _outactors_2
              (message `/Game/UI/Score_Interface.HighScore` _array_element_3 false)
              (`KismetSystemLibrary.PrintString` "nice")
              (if (== (`self.IngredientCount`) (`self.NeededIngredients`)) :!label _label_4
                (set `self.IngredientCount` 0)
                (if (== (`KismetArrayLibrary.Array_LastIndex` (`self.CurrentRecipe`)) -1)
                  (`KismetSystemLibrary.PrintString` "RECIPE COMPLETED")
                  (else
                    (`KismetSystemLibrary.PrintString` "fuck you")))
                (`self.CustomEvent_0`)
                (`KismetSystemLibrary.PrintString` "SEDRFTGYUHIJMOK,PL.Ö")))
            (else
              (`KismetSystemLibrary.PrintString` "boo")
              (goto _label_4))))
        (:`then_1`
          (`self.K2_DestroyActor` OtherActor)
          (goto _label_3 :!via `Reset`))))))

(fn `UserConstructionScript`)